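; BP_Checkpoint is a respawn checkpoint that activates when the main character overlaps its collision box.
; On overlap it passes its Arrow's world transform and a self-reference to GM_MyGameMode as the new respawn point, then swaps the push-button mesh to an alternate material.
; A separate ReturnCheckpointToNormal event restores the default button material.
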(event OnComponentBeginOverlap(CollisionBox)
  (params (OverlappedComponent :type Primitive%20Component%20Object%20Reference) (OtherActor :type Actor%20Object%20Reference) (OtherComp :type Primitive%20Component%20Object%20Reference) (OtherBodyIndex :type Integer) (bFromSweep :type Boolean) (SweepResult :type Hit%20Result%20Structure%20%28by%20ref%29))
  (Utilities|Casting|CastToBP_MainCharacter OtherActor)
  (bind _asgm_my_game_mode (Utilities|Casting|CastToGM_MyGameMode (Game|GetGameMode)))
  (Default|UpadateRespawnPoint _asgm_my_game_mode (Transformation|GetWorldTransform (Variables|Default|GetArrow)) self)
  (Rendering|Material|SetMaterial (Variables|Default|GetSM_PushButton) 0 "/Game/TeachersMarketplace/Assets/Props/Buttons/Button_A/Material/M_Button_A_2.M_Button_A_2"))

(event Custom|Return%20Checkpoint%20To%20Normal
  (Rendering|Material|SetMaterial (Variables|Default|GetSM_PushButton) 0 "/Game/TeachersMarketplace/Assets/Props/Buttons/Button_A/Material/M_Button_A.M_Button_A"))

(fn ConstructionScript)