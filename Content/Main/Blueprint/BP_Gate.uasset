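; BP_Gate is a force-field gate that the player character unlocks by spending a blue or red key.
; Entering the collision box checks the GateType gameplay tag (anything other than Key.Blue uses red), then decrements the matching key count and updates the HUD.
; Opening disables force-field collision and runs a timeline that drives Opacity on a dynamic material instance, marking the gate open to prevent reuse.
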(event OnComponentBeginOverlap(CollisionBox)
  (params (OverlappedComponent :type Primitive%20Component%20Object%20Reference) (OtherActor :type Actor%20Object%20Reference) (OtherComp :type Primitive%20Component%20Object%20Reference) (OtherBodyIndex :type Integer) (bFromSweep :type Boolean) (SweepResult :type Hit%20Result%20Structure%20%28by%20ref%29))
  ;[1 0.5236 0.7497] Event Overlap
  (bind _asbp_main_character (Utilities|Casting|CastToBP_MainCharacter OtherActor))
  (Variables|Default|SetBP%20MainCharacter_Ref _asbp_main_character)
  (if (GameplayTags|HasTag (Variables|Default|GetGateType) "(TagName=\"Key.Blue\")" true)
    (bind _bp_maincharacter_ref (Variables|Default|GetBP%20MainCharacter_Ref)
      (:then
        (if (> (Variables|/Game/Main/Player/BP_MainCharacter.BP_MainCharacter_C|GetNoOfBlueKeys _bp_maincharacter_ref) 0)
          (if (not (Variables|Default|GetIsOpen?))
            (CallFunction|OpentheGate)
            (bind _output_get (Variables|/Game/Main/Player/BP_MainCharacter.BP_MainCharacter_C|SetNoOfBlueKeys _bp_maincharacter_ref (- (Variables|/Game/Main/Player/BP_MainCharacter.BP_MainCharacter_C|GetNoOfBlueKeys _bp_maincharacter_ref) 1)))
            (Variables|/Game/Main/UI/UI_HUD.UI_HUD_C|SetNoOfBlueKeysToDisplay (Variables|/Game/Main/Player/BP_MainCharacter.BP_MainCharacter_C|GetHUDRef _bp_maincharacter_ref) _output_get))))
      (:else))
    (else
      (bind _bp_maincharacter_ref_2 (Variables|Default|GetBP%20MainCharacter_Ref)
        (:then
          (if (> (Variables|/Game/Main/Player/BP_MainCharacter.BP_MainCharacter_C|GetNoOfRedKeys _bp_maincharacter_ref_2) 0)
            (if (not (Variables|Default|GetIsOpen?))
              (CallFunction|OpentheGate)
              (bind _output_get_2 (Variables|/Game/Main/Player/BP_MainCharacter.BP_MainCharacter_C|SetNoOfRedKeys _bp_maincharacter_ref_2 (- (Variables|/Game/Main/Player/BP_MainCharacter.BP_MainCharacter_C|GetNoOfRedKeys _bp_maincharacter_ref_2) 1)))
              (Variables|/Game/Main/UI/UI_HUD.UI_HUD_C|SetNoOfRedKeysToDisplay (Variables|/Game/Main/Player/BP_MainCharacter.BP_MainCharacter_C|GetHUDRef _bp_maincharacter_ref_2) _output_get_2))))
        (:else)))))

(event Custom|OpenTheGate
  ;[0.5828 0.5207 1] Open The Gate
  (Collision|SetCollisionEnabled (Variables|Default|GetSM_ForceField) "NoCollision")
  (bind _dooropen (Timeline|DoorOpen Play)
    (:Update
      (Rendering|Material|SetScalarParameterValue (Variables|Default|GetForceFieldReference) "Opacity" _dooropen :!class /Script/Engine.MaterialInstanceDynamic)
      (Variables|Default|SetIsOpen? true))))

(event EventBeginPlay
  (bind _returnvalue (Game|GetGameMode))
  ;[1 1 1] Event Begin Play
  (bind _returnvalue_2 (Rendering|Material|CreateDynamicMaterialInstance (Variables|Default|GetSM_ForceField) 0 0 "None" :!class /Script/Engine.PrimitiveComponent))
  (Variables|Default|SetForceFieldReference _returnvalue_2)
  (Utilities|IsValid _returnvalue
    (:Is%20Valid
      (bind _asgm_my_game_mode (Utilities|Casting|CastToGM_MyGameMode _returnvalue)
        (:then
          (Utilities|IsValid _asgm_my_game_mode
            (:Is%20Valid
              (Variables|Default|SetHUDReference (Variables|/Game/Main/GameSettings/GM_MyGameMode.GM_MyGameMode_C|GetHUDRef _asgm_my_game_mode)))))
        (:CastFailed
          (Development|PrintString "cast failed"))))
    (:Is%20Not%20Valid
      (Development|PrintString "GM null"))))

(fn ConstructionScript)