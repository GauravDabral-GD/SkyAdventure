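; Game mode that runs the game flow: main menu, lives, checkpoint respawning, and win and game-over screens.
; On start it takes the respawn point from a PlayerStart and creates the HUD and main menu; checkpoints replace that point and reset the previous one.
; Death costs a life and always teleports the character back, refreshing HUD health, then triggers game over when no lives remain.
; Menu and end screens switch input to UI-only with a cursor.
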(event Custom|WinGame
  (bind _returnvalue (Game|GetPlayerController 0))
  (bind _asbp_main_character (Utilities|Casting|CastToBP_MainCharacter (Game|GetPlayerCharacter 0)))
  (Default|EnterCelebration _asbp_main_character)
  (bind _returnvalue_2 (UserInterface|CreateWidget "/Game/Main/UI/UI_WinDisplay.UI_WinDisplay_C"))
  (UserInterface|Viewport|AddtoViewport _returnvalue_2 0)
  (Variables|/Script/Engine.PlayerController|SetbShowMouseCursor _returnvalue true)
  (Input|SetInputModeUIOnly _returnvalue 0 "DoNotLock" false))

(event Custom|Death
  (params (PlayerCharacter :type Character%20Object%20Reference))
  ;[1 1 1] Death and Respawn
  (bind _asbp_main_character (Utilities|Casting|CastToBP_MainCharacter PlayerCharacter))
  (bind _output_get (Variables|/Game/Main/Player/BP_MainCharacter.BP_MainCharacter_C|SetLives _asbp_main_character (- (Variables|/Game/Main/Player/BP_MainCharacter.BP_MainCharacter_C|GetLives _asbp_main_character) 1)))
  (if (<= _output_get 0)
    (CallFunction|Respawn _asbp_main_character)
    (CallFunction|LoseGame)
    (else
      (CallFunction|Respawn _asbp_main_character))))

(event Custom|Respawn
  (params (Player :type Actor%20Object%20Reference))
  (bind _respawnpoint (Variables|Default|GetRespawnPoint))
  ;[1 1 1] Death and Respawn
  (Transformation|Teleport Player (.location _respawnpoint) (.rotation _respawnpoint))
  (bind _hudref (Variables|Default|GetHUDRef)
    (:then
      (Default|DisplayHealth _hudref))
    (:else)))

(event Custom|LoseGame
  (bind _returnvalue (Game|GetPlayerController 0))
  (bind _returnvalue_2 (UserInterface|CreateWidget "/Game/Main/UI/UI_GameOverDisplay.UI_GameOverDisplay_C"))
  (UserInterface|Viewport|AddtoViewport _returnvalue_2 0)
  (Variables|/Script/Engine.PlayerController|SetbShowMouseCursor _returnvalue true)
  (Input|SetInputModeUIOnly _returnvalue 0 "DoNotLock" false))

(event EventBeginPlay
  (bind _returnvalue (Game|GetPlayerController 0))
  (bind _returnvalue_2 (Actor|GetActorOfClass "/Script/Engine.PlayerStart"))
  (Variables|Default|SetRespawnPoint (Transformation|GetActorTransform _returnvalue_2))
  (bind _returnvalue_3 (UserInterface|CreateWidget "/Game/Main/UI/UI_HUD.UI_HUD_C"))
  (bind _output_get (Variables|Default|SetHUDRef _returnvalue_3))
  (UserInterface|Viewport|AddtoViewport _output_get -1)
  (bind _returnvalue_4 (UserInterface|CreateWidget "/Game/Main/UI/UI_MainMenu.UI_MainMenu_C"))
  (UserInterface|Viewport|AddtoViewport _returnvalue_4 0)
  (Variables|/Script/Engine.PlayerController|SetbShowMouseCursor _returnvalue true)
  (Input|SetInputModeUIOnly _returnvalue 0 "DoNotLock" false))

(fn ConstructionScript)

(fn UpadateRespawnPoint
  (params (RespawnPoint :type Transform) (Checkpoint%20Ref :type BP%20Checkpoint%20Object%20Reference))
  (Utilities|FlowControl|Sequence
    (:then_0
      (if (Utilities|IsValid (Variables|Default|GetCurrent%20Checkpoint%20Ref))
        (Default|ReturnCheckpointtoNormal (Variables|Default|GetCurrent%20Checkpoint%20Ref))))
    (:then_1
      (Variables|Default|SetRespawnPoint RespawnPoint)
      (Variables|Default|SetCurrent%20Checkpoint%20Ref Checkpoint%20Ref))))